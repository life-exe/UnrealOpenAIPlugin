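; BP_APIOverview is a reference Blueprint that lays out the nodes of an OpenAI API plugin and does nothing at runtime.
; Disconnected examples, mostly grouped by endpoint, cover completions, embeddings, images, audio, files, uploads, batches, models, moderation, fine-tuning and assistants.
; Each pairs request nodes with Make-struct inputs, and many expose response fields through loops or unused pins.
; It also shows helper nodes for enum-to-string conversion, token loading, file handling and texture creation.
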(fn ConstructionScript)